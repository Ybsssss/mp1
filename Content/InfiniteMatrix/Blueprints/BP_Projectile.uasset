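; BP_Projectile is a player projectile that kills enemies on contact and awards score.
; When its ProjectileHit component overlaps a BP_Enemy, it destroys that enemy, adds points to the Score on player pawn 0's BP_Player, then destroys itself.
; It also pushes the truncated score straight to the player's ScoreWidget.
; Overlaps with other actors are ignored, and the mesh hit event is empty.
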(event `self.ProjectileMesh.OnComponentHit`
  (params (HitComponent :type "PrimitiveComponent Object Reference") (OtherActor :type "Actor Object Reference") (OtherComp :type "PrimitiveComponent Object Reference") (NormalImpulse :type "Vector Structure") (Hit :type "HitResult Structure (by ref)")))

(event `self.ProjectileHit.OnComponentBeginOverlap`
  (params (OverlappedComponent :type "PrimitiveComponent Object Reference") (OtherActor :type "Actor Object Reference") (OtherComp :type "PrimitiveComponent Object Reference") (OtherBodyIndex :type Integer) (bFromSweep :type Boolean) (SweepResult :type "HitResult Structure (by ref)"))
  (bind _asbp_enemy (cast `/Game/InfiniteMatrix/Blueprints/BP_Enemy` OtherActor))
  (`self.K2_DestroyActor` _asbp_enemy)
  (bind _asbp_player (cast `/Game/InfiniteMatrix/Blueprints/BP_Player` (`GameplayStatics.GetPlayerPawn` 0)))
  (bind _output_get (set `/Game/InfiniteMatrix/Blueprints/BP_Player.Score` (+ (`/Game/InfiniteMatrix/Blueprints/BP_Player.Score` _asbp_player) 5.0) _asbp_player))
  (`self.K2_DestroyActor`)
  (`/Game/InfiniteMatrix/UI/WBP_Score.UpdateText` (`/Game/InfiniteMatrix/Blueprints/BP_Player.ScoreWidget` _asbp_player) (`KismetMathLibrary.FTrunc` _output_get)))

(fn `UserConstructionScript`)